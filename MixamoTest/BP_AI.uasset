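; BP_AI is an AI-controlled pawn that moves toward actors it detects and can roam at random.
; PawnSensing hear and see events issue AIMoveTo toward the noise instigator or seen pawn, then start a retriggerable delay that leads nowhere.
; RandomRoam moves to a random reachable nearby point and calls itself again on success.
; Nothing in this graph calls RandomRoam, including after a chase.
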(event OnSeePawn(PawnSensing)
  (params (Pawn :type Pawn%20Object%20Reference))
  (Utilities|FlowControl|Sequence
    (:then_0
      (AI|AIMoveTo self "0, 0, 0" Pawn 5.0 false))
    (:then_1
      (Utilities|FlowControl|RetriggerableDelay 1.0))))

(event OnHearNoise(PawnSensing)
  (params (Instigator :type Pawn%20Object%20Reference) (Location :type Vector%20%28by%20ref%29 :default "0, 0, 0") (Volume :type Float%20%28single-precision%29))
  (Utilities|FlowControl|Sequence
    (:then_0
      (AI|AIMoveTo self "0, 0, 0" Instigator 5.0 false))
    (:then_1
      (Utilities|FlowControl|RetriggerableDelay 1.0))))

(event Custom|Random%20Roam
  ;[1 1 1] Fonction pour faire avancer aléatoirement le personnage
  (AI|AIMoveTo self (.RandomLocation (AI|Navigation|GetRandomReachablePointinRadius (Transformation|GetActorLocation) 1.5e+03 0 0)) 0 5.0 false
    (:OnSuccess
      (CallFunction|RandomRoam))))

(fn ConstructionScript)